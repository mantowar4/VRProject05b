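; BP_StairUp is a stair actor with a widget that labels it as a way to go up or down.
; On BeginPlay it passes its Location and Rotation values to the w_Stairs widget.
; EnumStairsWidget selects the Russian "descend" or "ascend" caption and the matching Down or UP arrow image, rebuilding the brush from the existing one.
; The Teleport event is an empty stub, so no movement happens in this Blueprint.
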(event `self.ReceiveBeginPlay`
  (bind _asw_stairs (cast `/Game/Widgets/w_Stairs` (`WidgetComponent.GetUserWidgetObject` (`self.Widget`))))
  (set `/Game/Widgets/w_Stairs.Location` (`self.Location`) _asw_stairs)
  (set `/Game/Widgets/w_Stairs.Rotation` (`self.Rotation`) _asw_stairs)
  (if (`|EnumEquality` (`self.enum_stairsWidget`) "NewEnumerator0")
    (bind _text (`/Game/Widgets/w_Stairs.Text` _asw_stairs))
    (`TextBlock.SetText` _text "Спуститься")
    (bind _image_41 (`/Game/Widgets/w_Stairs.Image_41` _asw_stairs))
    (bind (_imagesize _margin _tintcolor _resourceobject _drawas _tiling _mirroring) (break `SlateBrush` (`Image.Brush` _image_41)))
    (`Image.SetBrush` _image_41 (make `SlateBrush` _imagesize _margin _tintcolor "/Game/Textures/Down.Down" _drawas _tiling _mirroring))
    (else
      (`TextBlock.SetText` _text "Подняться")
      (`Image.SetBrush` _image_41 (make `SlateBrush` _imagesize _margin (struct :`SpecifiedColor` (struct :`R` 1.0 :`G` 1.0 :`B` 1.0 :`A` 1.0) :`ColorUseRule` "UseColor_Specified") "/Game/Textures/UP.UP" _drawas _tiling _mirroring)))))

(event `Teleport`)

(fn `UserConstructionScript`)